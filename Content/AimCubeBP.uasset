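; AimCubeBP is a cube actor, apparently an aim-practice target, that activates cubes by setting their scale to one.
; On BeginPlay, each instance caches all AimCubeBP actors in an array and sets the first to unit scale.
; On Hit, it sets a randomly picked cube from that array, possibly itself, to unit scale.
; The graph never scales any cube back down.
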(event `self.ReceiveBeginPlay`
  (bind _outactors (`GameplayStatics.GetAllActorsOfClass` "AimCubeBP_C"))
  (bind _output_get (set `self.AimCubes` _outactors))
  (`SceneComponent.SetWorldScale3D` (`Actor.RootComponent` (`|GetArrayItem` _output_get)) (1.0 1.0 1.0)))

(event `self.ReceiveHit`
  (params (MyComp :type "PrimitiveComponent Object Reference") (Other :type "Actor Object Reference") (OtherComp :type "PrimitiveComponent Object Reference") (bSelfMoved :type Boolean) (HitLocation :type "Vector Structure") (HitNormal :type "Vector Structure") (NormalImpulse :type "Vector Structure") (Hit :type "HitResult Structure (by ref)"))
  (bind _aimcubes (`self.AimCubes`))
  (`SceneComponent.SetWorldScale3D` (`Actor.RootComponent` (`|GetArrayItem` _aimcubes (`KismetMathLibrary.RandomInteger` (`KismetArrayLibrary.Array_Length` _aimcubes)))) (1.0 1.0 1.0)))

(fn `UserConstructionScript`)